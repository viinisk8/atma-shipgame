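; Game mode for Atma that sets up the player's UI and keeps the score display current.
; On BeginPlay it adds the HUD to the viewport, installs a custom cursor widget for the first player and caches the Atma game instance.
; Every tick it copies the Victories and Defeats counts from that game instance into the HUD's score text.
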(event `self.ReceiveBeginPlay`
  (bind _returnvalue (`GameplayStatics.GetPlayerController` 0))
  ;[1 1 1] Create HUD
  (bind _returnvalue_2 (`|CreateWidget` "/Game/HUD/HUD.HUD_C"))
  (bind _output_get (set `self.HUD` _returnvalue_2))
  (`UserWidget.AddToViewport` _output_get 0)
  ;[1 1 1] Set Cursor
  (bind _returnvalue_3 (`|CreateWidget` "/Game/HUD/Cursor.Cursor_C"))
  (`PlayerController.SetMouseCursorWidget` _returnvalue "Default" _returnvalue_3)
  (set `PlayerController.bShowMouseCursor` true _returnvalue)
  ;[1 1 1] GameInstanceRef
  (`self.GetGameInstanceRef`))

(event `self.ReceiveTick`
  (params (DeltaSeconds :type "Float (single-precision)"))
  (bind _as_bp_atma_game_instance (`self.As BP Atma Game Instance`))
  (bind _score (`/Game/HUD/HUD.Score` (`self.HUD`)))
  ;[1 1 1] Set Score
  (`/Engine/EditorBlueprintResources/StandardMacros.IsValid` _as_bp_atma_game_instance
    (:`Is Valid`
      (`TextBlock.SetText` (`/Game/HUD/Score.victories` _score) (`KismetTextLibrary.Conv_IntToText` (`/Game/GameInstance/BP_AtmaGameInstance.Victories` _as_bp_atma_game_instance)))
      (`TextBlock.SetText` (`/Game/HUD/Score.defeats` _score) (`KismetTextLibrary.Conv_IntToText` (`/Game/GameInstance/BP_AtmaGameInstance.Defeats` _as_bp_atma_game_instance))))))

(fn `GetGameInstanceRef`
  (bind _asbp_atma_game_instance (cast `/Game/GameInstance/BP_AtmaGameInstance` (`GameplayStatics.GetGameInstance`)))
  (set `self.As BP Atma Game Instance` _asbp_atma_game_instance))

(fn `UserConstructionScript`)