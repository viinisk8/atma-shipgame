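; Player controller for the player ship, turning Enhanced Input and mouse clicks into movement and shooting.
; BeginPlay adds the input mapping context and caches the BP_PlayerShip pawn.
; Tick rotates the ship and applies a slight constant Y movement when that axis is idle.
; Left click deprojects the cursor to world space and passes a Y-flattened direction to the ship's WeaponSystem to fire.
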(event `self.ReceiveTick`
  (params (DeltaSeconds :type "Float (single-precision)"))
  ;[1 1 1] RotateSystem
  (`self.RotateShip`)
  ;[1 1 1] MoveShipToUp
  (if (== (`|GetInputActionValue`) 0.0)
    (`self.AddMovementY` 0.2)))

(event `self.ReceiveBeginPlay`
  ;[1 1 1] AddMapping
  (message `EnhancedInputSubsystemInterface.AddMappingContext` (pcsubsystem `EnhancedInputLocalPlayerSubsystem` self) "/Game/Player/Inputs/AtmaInputMappingContext.AtmaInputMappingContext" 0 (struct))
  ;[1 1 1] Create Player Reference
  (bind _asbp_player_ship (cast `/Game/Player/BP_PlayerShip` (`GameplayStatics.GetPlayerPawn` 0)))
  (set `self.As BP Player Ship` _asbp_player_ship))

(event `EnhancedInput|/Game/Player/Inputs/IA_MoveY`
  (params (ActionValue :type "Float (double-precision)") (ElapsedSeconds :type "Float (double-precision)") (TriggeredSeconds :type "Float (double-precision)") (InputAction :type "InputAction Object Reference" :default "/Game/Player/Inputs/IA_MoveY.IA_MoveY"))
  ;[1 1 1] AddMovementY
  (:`Triggered`
    (`self.AddMovementY` ActionValue)))

(event `EnhancedInput|/Game/Player/Inputs/IA_MoveX`
  (params (ActionValue :type "Float (double-precision)") (ElapsedSeconds :type "Float (double-precision)") (TriggeredSeconds :type "Float (double-precision)") (InputAction :type "InputAction Object Reference" :default "/Game/Player/Inputs/IA_MoveX.IA_MoveX"))
  ;[1 1 1] AddMovementX
  (:`Triggered`
    (`self.AddMovementX` ActionValue)))

(event `Key|LeftMouseButton`
  (params (Key :type "Key Structure"))
  (bind (_locationx _locationy) (`self.GetMousePosition`))
  (bind _returnvalue (`self.K2_GetActorLocation` (`self.K2_GetPawn`)))
  ;[1 1 1] shooting
  (:`Pressed`
    (`WeaponSystem.HandleFire` (`/Game/Player/BP_PlayerShip.WeaponSystem` (`self.As BP Player Ship`)) _returnvalue (`KismetMathLibrary.MakeVector` (.x (- (`self.DeprojectScreenPositionToWorld` _locationx _locationy) _returnvalue)) 0.0 (.z (- (`self.DeprojectScreenPositionToWorld` _locationx _locationy) _returnvalue))))))

(fn `SetCursorByState`
  (params (StateOfShip :type "EStateOfShip Enum" :default "Ready")))

(fn `UserConstructionScript`)